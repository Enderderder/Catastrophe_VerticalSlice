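; Spline-driven fence tool for the Hub kitset that lays out fence meshes along an editable spline.
; The construction script divides the spline length by Spacing and adds an SM_Hub_Fence component with the Lambert1 material at each interval.
; Each piece follows the spline's local position and rotation, with yaw turned a quarter turn to align the mesh.
; The event graph has no active runtime logic.
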(event EventBeginPlay)

(event Collision|EventActorBeginOverlap
  (params (OtherActor :type Actor%20Object%20Reference)))

(event EventTick
  (params (DeltaSeconds :type Float%20%28single-precision%29)))

(fn ConstructionScript
  (bind _splinecomponentexample (Variables|Default|GetSplineComponentExample))
  (bind _spacing (Variables|Default|Getspacing))
  (for _index (range 0 (.ReturnValue (Math|Float|Division(WholeandRemainder) (Spline|GetSplineLength _splinecomponentexample) _spacing)))
    (bind _returnvalue (AddComponent|AddStaticMeshComponent false (Math|Transform|MakeTransform (Spline|GetLocationatDistanceAlongSpline _splinecomponentexample (* _index _spacing) "Local") (Math|Rotator|MakeRotator (.roll (Spline|GetRotationatDistanceAlongSpline _splinecomponentexample (* _index _spacing) "Local")) (.pitch (Spline|GetRotationatDistanceAlongSpline _splinecomponentexample (* _index _spacing) "Local")) (+ (.yaw (Spline|GetRotationatDistanceAlongSpline _splinecomponentexample (* _index _spacing) "Local")) 9e+01)))))
    (Components|StaticMesh|SetStaticMesh _returnvalue "/Game/Assets/Kitsets/Kitset_Hub/SM_Hub_Fence.SM_Hub_Fence")
    (Rendering|Material|SetMaterial _returnvalue 0 "/Game/Assets/Kitsets/Kitset_Jail/Props/lambert1.lambert1")))