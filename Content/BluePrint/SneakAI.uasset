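; AI controller for an EnemyMele guard in a stealth setup, running the SneakTree behavior tree on possession.
; Sight perception writes player visibility and alert state to the SneakBoard blackboard, treating a Hidden player as unseen.
; State events (walk, run, spotted, alert, looking, stun) forward to the guard pawn and sync blackboard keys like stun and last known player location.
; Alert clears after a countdown of calls, and stun temporarily disables sight.
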(event OnTargetPerceptionUpdated(AIPerception)
  (params (Actor :type Actor%20Object%20Reference) (Stimulus :type AI%20Stimulus%20Structure))
  (bind _bsuccessfullysensed (Utilities|Struct|BreakAIStimulus Stimulus))
  ;[1 1 1] Using the sight Perception
  (Utilities|Casting|CastToPlayerCharacter Actor)
  (if (Variables|/Script/Engine.Actor|GetbHidden (Game|GetPlayerCharacter 0))
    (AI|Components|Blackboard|SetValueasBool (AI|GetBlackboard 0) (Utilities|Name|MakeLiteralName "CanSeePlayer") false)
    (else
      (AI|Components|Blackboard|SetValueasBool (AI|GetBlackboard 0) (Utilities|Name|MakeLiteralName "CanSeePlayer") _bsuccessfullysensed)
      (if _bsuccessfullysensed
        (bind _blackboardcomponent (Class|AIController|UseBlackboard "/Game/BluePrint/SneakBoard.SneakBoard"))
        (AI|Components|Blackboard|SetValueasBool _blackboardcomponent (Utilities|Name|MakeLiteralName "Alert") true)))))

(event Custom|Walk
  (bind _guard (Variables|Default|GetGuard))
  (if (Variables|/Game/BluePrint/EnemyMele.EnemyMele_C|GetIsStationary _guard)
    (CallFunction|ReturntoStationaryPoint)
    (else
      (Default|Walk _guard)
      (bind _blackboardcomponent (Class|AIController|UseBlackboard "/Game/BluePrint/SneakBoard.SneakBoard"))
      (AI|Components|Blackboard|SetValueasBool _blackboardcomponent (Utilities|Name|MakeLiteralName "IsStun") (Variables|/Game/BluePrint/EnemyMele.EnemyMele_C|GetIsStun _guard)))))

(event Custom|Run
  (bind _guard (Variables|Default|GetGuard))
  (Default|Run _guard)
  (bind _blackboardcomponent (Class|AIController|UseBlackboard "/Game/BluePrint/SneakBoard.SneakBoard"))
  (AI|Components|Blackboard|SetValueasBool _blackboardcomponent (Utilities|Name|MakeLiteralName "IsStun") (Variables|/Game/BluePrint/EnemyMele.EnemyMele_C|GetIsStun _guard))
  (if (Variables|/Script/Engine.Actor|GetbHidden (Game|GetPlayerCharacter 0))
    (AI|Components|Blackboard|SetValueasBool (AI|GetBlackboard 0) (Utilities|Name|MakeLiteralName "CanSeePlayer") false)
    (elif (not (.bSuccessfullySensed (Utilities|Struct|BreakAIStimulus (stale OnTargetPerceptionUpdated(AIPerception) Stimulus))))
      (Utilities|FlowControl|Delay 1.0)
      (bind _blackboardcomponent_2 (Class|AIController|UseBlackboard "/Game/BluePrint/SneakBoard.SneakBoard"))
      (AI|Components|Blackboard|SetValueasVector _blackboardcomponent_2 (Utilities|Name|MakeLiteralName "LastKnownPlayerLocation") (Transformation|GetActorLocation (Game|GetPlayerCharacter 0))))))

(event Custom|Alert
  (bind _guard (Variables|Default|GetGuard))
  (Default|Alert _guard)
  (bind _blackboardcomponent (Class|AIController|UseBlackboard "/Game/BluePrint/SneakBoard.SneakBoard"))
  (AI|Components|Blackboard|SetValueasBool _blackboardcomponent (Utilities|Name|MakeLiteralName "IsStun") (Variables|/Game/BluePrint/EnemyMele.EnemyMele_C|GetIsStun _guard))
  (bind _result (Math|Integer|DecrementInt (Variables|Default|GetStopSeekCount))
    (:%20%20
      (if (<= _result 0)
        (bind _blackboardcomponent_2 (Class|AIController|UseBlackboard "/Game/BluePrint/SneakBoard.SneakBoard"))
        (AI|Components|Blackboard|SetValueasBool _blackboardcomponent_2 (Utilities|Name|MakeLiteralName "Alert") false)
        (Variables|Default|SetStopSeekCount 2)))))

(event Custom|Looking
  (bind _guard (Variables|Default|GetGuard))
  (Default|Looking _guard)
  (bind _blackboardcomponent (Class|AIController|UseBlackboard "/Game/BluePrint/SneakBoard.SneakBoard"))
  (AI|Components|Blackboard|SetValueasBool _blackboardcomponent (Utilities|Name|MakeLiteralName "IsStun") (Variables|/Game/BluePrint/EnemyMele.EnemyMele_C|GetIsStun _guard)))

(event Custom|Stun
  (bind _aiperception (Variables|Default|GetAIPerception))
  (Default|Stun (Variables|Default|GetGuard))
  (Class|AIPerceptionComponent|SetSenseEnabled _aiperception "/Script/AIModule.AISense_Sight" false)
  (Utilities|FlowControl|Delay 5.0)
  (Class|AIPerceptionComponent|SetSenseEnabled _aiperception "/Script/AIModule.AISense_Sight" true)
  (bind _blackboardcomponent (Class|AIController|UseBlackboard "/Game/BluePrint/SneakBoard.SneakBoard"))
  (AI|Components|Blackboard|SetValueasBool _blackboardcomponent (Utilities|Name|MakeLiteralName "IsStun") false))

(event Custom|Spoted
  (bind _returnvalue (AI|GetBlackboard 0))
  (Default|Spoted (Variables|Default|GetGuard))
  (AI|Components|Blackboard|SetValueasVector _returnvalue (Utilities|Name|MakeLiteralName "LastKnownPlayerLocation") (Transformation|GetActorLocation (Game|GetPlayerCharacter 0)))
  (Utilities|FlowControl|Delay (Variables|Default|GetDelayTime))
  (AI|Components|Blackboard|SetValueasBool _returnvalue (Utilities|Name|MakeLiteralName "Spoted") true)
  (if (not (ScalableFloat|GetValueasBool _returnvalue (Utilities|Name|MakeLiteralName "CanSeePlayer")))
    (CallFunction|Alert)))

(event Custom|Return%20to%20Stationary%20Point
  (Default|ReturntoStationaryPoint (Variables|Default|GetGuard)))

(event EventBeginPlay
  (AI|Components|Blackboard|SetValueasBool (AI|GetBlackboard 0) (Utilities|Name|MakeLiteralName "IsStationary") (Variables|/Game/BluePrint/EnemyMele.EnemyMele_C|GetIsStationary (Variables|Default|GetGuard))))

(event EventOnPossess
  (params (PossessedPawn :type Pawn%20Object%20Reference))
  (bind _asenemy_mele (Utilities|Casting|CastToEnemyMele PossessedPawn))
  (Variables|Default|SetGuard _asenemy_mele)
  (AI|RunBehaviorTree "/Game/BluePrint/SneakTree.SneakTree"))

(fn ConstructionScript)