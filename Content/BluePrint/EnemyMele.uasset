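; Melee guard enemy for a stealth game that patrols waypoints, chases the player and restarts the level on touch unless stunned or the player is hidden.
; State events, not called within this graph, set walk speed, spotlight color and guard, alert and question-mark animation flags, using AIMoveTo for movement.
; Tomatoes hitting Stunarea set IsStun, which Looking turns into a timed stun, while the NotStun volume destroys them.
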(event OnComponentBeginOverlap(notStun)
  (params (OverlappedComponent :type Primitive%20Component%20Object%20Reference) (OtherActor :type Actor%20Object%20Reference) (OtherComp :type Primitive%20Component%20Object%20Reference) (OtherBodyIndex :type Integer) (bFromSweep :type Boolean) (SweepResult :type Hit%20Result%20Structure%20%28by%20ref%29))
  (bind _asbp_tomato (Utilities|Casting|CastToBP_Tomato OtherActor))
  (Actor|DestroyActor _asbp_tomato))

(event OnComponentBeginOverlap(stunarea)
  (params (OverlappedComponent :type Primitive%20Component%20Object%20Reference) (OtherActor :type Actor%20Object%20Reference) (OtherComp :type Primitive%20Component%20Object%20Reference) (OtherBodyIndex :type Integer) (bFromSweep :type Boolean) (SweepResult :type Hit%20Result%20Structure%20%28by%20ref%29))
  (Utilities|Casting|CastToBP_Tomato OtherActor)
  (if (not (Variables|Default|GetIsStun))
    (Variables|Default|SetIsStun true)
    (Effects|SpawnEmitteratLocation "/Game/VFX/Stun_VFX.Stun_VFX" (Transformation|GetWorldLocation (Variables|Default|GetStunVFX)))
    (Audio|PlaySound2D "/Game/Sound/GORE_Splat_Hit_Bubbles_mono_Cue.GORE_Splat_Hit_Bubbles_mono_Cue" 1.0 1.0 0.0 0 0)))

(event OnComponentHit(CapsuleComponent)
  (params (HitComponent :type Primitive%20Component%20Object%20Reference) (OtherActor :type Actor%20Object%20Reference) (OtherComp :type Primitive%20Component%20Object%20Reference) (NormalImpulse :type Vector :default "0, 0, 0") (Hit :type Hit%20Result%20Structure%20%28by%20ref%29))
  ;[1 1 1] When player touch the enemy and restart the level
  (if (not (Variables|Default|GetIsStun))
    (if (not (Variables|/Script/Engine.Actor|GetbHidden (Game|GetPlayerCharacter 0)))
      (Utilities|Casting|CastToPlayerCharacter OtherActor)
      (bind _returnvalue (Game|GetCurrentLevelName true))
      (Game|OpenLevel(byName) (Utilities|String|StringToName _returnvalue)))))

(event Custom|Alert
  ;[1 1 1] when enemy is looking for player at their last known location
  (Variables|/Script/Engine.CharacterMovementComponent|SetMaxWalkSpeed (Variables|Character|GetCharacterMovement) (Variables|Default|GetAlert%20Speed))
  (Rendering|Components|Light|SetLightColor (Variables|Default|GetSpotLight1) (Math|Conversions|ToLinearColor(Color) (Variables|Default|GetSpot)) true)
  (Variables|/Game/Assets/Alert/Questionmark/QuestionMark_ABP.QuestionMark_ABP_C|SetbIsQuestion (Variables|Default|GetQuestionMarkABP_Ref) true)
  (Variables|/Game/Assets/Alert/Alert_ABP.Alert_ABP_C|SetIsAlert (Variables|Default|GetAlertABP_Ref) false))

(event Custom|Walk
  (bind _waypoint (Variables|Default|GetWayPoint))
  (bind _guardabp_ref (Variables|Default|GetGuardABP_Ref))
  ;[1 1 1] Enemy just moving towards the given waypoint
  (Variables|/Game/Assets/Alert/Questionmark/QuestionMark_ABP.QuestionMark_ABP_C|SetbIsQuestion (Variables|Default|GetQuestionMarkABP_Ref) false)
  (Variables|/Game/Assets/GuardAssets/Guard_ABP.Guard_ABP_C|SetIsRunning _guardabp_ref false)
  (Variables|/Game/Assets/GuardAssets/Guard_ABP.Guard_ABP_C|SetbWalking _guardabp_ref true)
  (Variables|/Script/Engine.CharacterMovementComponent|SetMaxWalkSpeed (Variables|Character|GetCharacterMovement) (Variables|Default|GetWalk%20Speed))
  (Rendering|Components|Light|SetLightColor (Variables|Default|GetSpotLight1) (Math|Conversions|ToLinearColor(Color) (Variables|Default|GetUnDetectedLight)) true)
  (Rendering|SetVisibility (Variables|Default|GetAlertMesh) true false)
  (AI|AIMoveTo self (Transformation|GetActorLocation (Utilities|Array|Get(acopy) _waypoint (Variables|Default|Getcount))) 0 1e+01 false
    (:OnSuccess
      (bind _result (Math|Integer|IncrementInt (Variables|Default|Getcount))
        (:%20%20
          (bind _output_get (Variables|Default|Setcount _result))
          (if (>= _output_get (Utilities|Array|Length _waypoint))
            (Variables|Default|Setcount 0)))))))

(event Custom|Spoted
  (bind _guardabp_ref (Variables|Default|GetGuardABP_Ref))
  ;[1 1 1] When Enemy is chasing Player
  (Variables|/Game/Assets/GuardAssets/Guard_ABP.Guard_ABP_C|SetIsSpoted _guardabp_ref true)
  (Variables|/Game/Assets/Alert/Questionmark/QuestionMark_ABP.QuestionMark_ABP_C|SetbIsQuestion (Variables|Default|GetQuestionMarkABP_Ref) true)
  (Variables|/Game/Assets/Alert/Alert_ABP.Alert_ABP_C|SetIsAlert (Variables|Default|GetAlertABP_Ref) false)
  (Variables|/Script/Engine.CharacterMovementComponent|SetMaxWalkSpeed (Variables|Character|GetCharacterMovement) 0.0)
  (Variables|/Game/Assets/GuardAssets/Guard_ABP.Guard_ABP_C|SetbWalking _guardabp_ref false)
  (Rendering|Components|Light|SetLightColor (Variables|Default|GetSpotLight1) (Math|Conversions|ToLinearColor(Color) (Variables|Default|GetSpot)) true))

(event Custom|Stun
  (bind _spotlight1 (Variables|Default|GetSpotLight1))
  (bind _guardabp_ref (Variables|Default|GetGuardABP_Ref))
  (Variables|/Game/Assets/GuardAssets/Guard_ABP.Guard_ABP_C|SetIsStunned _guardabp_ref true)
  (Variables|/Game/Assets/Alert/Alert_ABP.Alert_ABP_C|SetIsAlert (Variables|Default|GetAlertABP_Ref) false)
  (Variables|/Game/Assets/Alert/Questionmark/QuestionMark_ABP.QuestionMark_ABP_C|SetbIsQuestion (Variables|Default|GetQuestionMarkABP_Ref) false)
  (Variables|/Script/Engine.CharacterMovementComponent|SetMaxWalkSpeed (Variables|Character|GetCharacterMovement) 0.0)
  (Rendering|SetVisibility _spotlight1 false false)
  (Utilities|FlowControl|Delay 5.0)
  (Rendering|SetVisibility _spotlight1 true false)
  (Variables|/Game/Assets/GuardAssets/Guard_ABP.Guard_ABP_C|SetIsStunned _guardabp_ref false)
  (Variables|Default|SetIsStun false))

(event Custom|Looking
  (bind _guardabp_ref (Variables|Default|GetGuardABP_Ref))
  ;[1 1 1] adding a pause function when reach a waypoint
  (if (Variables|Default|GetIsStun)
    (CallFunction|Stun)
    (else
      (Variables|/Script/Engine.CharacterMovementComponent|SetMaxWalkSpeed (Variables|Character|GetCharacterMovement) 0.0)
      (Rendering|Components|Light|SetLightColor (Variables|Default|GetSpotLight1) (Math|Conversions|ToLinearColor(Color) (Variables|Default|GetUnDetectedLight)) true)
      (Variables|/Game/Assets/Alert/Questionmark/QuestionMark_ABP.QuestionMark_ABP_C|SetbIsQuestion (Variables|Default|GetQuestionMarkABP_Ref) false)
      (Variables|/Game/Assets/Alert/Alert_ABP.Alert_ABP_C|SetIsAlert (Variables|Default|GetAlertABP_Ref) false)
      (Variables|/Game/Assets/GuardAssets/Guard_ABP.Guard_ABP_C|SetIsRunning _guardabp_ref false)
      (Variables|/Game/Assets/GuardAssets/Guard_ABP.Guard_ABP_C|SetbWalking _guardabp_ref false)
      (Variables|/Game/Assets/GuardAssets/Guard_ABP.Guard_ABP_C|SetIsLooking _guardabp_ref true)
      (Utilities|FlowControl|Delay 1.0)
      (Variables|/Game/Assets/GuardAssets/Guard_ABP.Guard_ABP_C|SetIsLooking _guardabp_ref false))))

(event Custom|Run
  (bind _guardabp_ref (Variables|Default|GetGuardABP_Ref))
  ;[1 1 1] When Enemy is chasing Player
  (Variables|/Game/Assets/GuardAssets/Guard_ABP.Guard_ABP_C|SetIsSpoted _guardabp_ref false)
  (Variables|/Game/Assets/Alert/Questionmark/QuestionMark_ABP.QuestionMark_ABP_C|SetbIsQuestion (Variables|Default|GetQuestionMarkABP_Ref) false)
  (Variables|/Game/Assets/Alert/Alert_ABP.Alert_ABP_C|SetIsAlert (Variables|Default|GetAlertABP_Ref) true)
  (Variables|/Script/Engine.CharacterMovementComponent|SetMaxWalkSpeed (Variables|Character|GetCharacterMovement) (Variables|Default|GetRun%20Speed))
  (Variables|/Game/Assets/GuardAssets/Guard_ABP.Guard_ABP_C|SetbWalking _guardabp_ref false)
  (Variables|/Game/Assets/GuardAssets/Guard_ABP.Guard_ABP_C|SetIsRunning _guardabp_ref true)
  (Rendering|Components|Light|SetLightColor (Variables|Default|GetSpotLight1) (Math|Conversions|ToLinearColor(Color) (Variables|Default|GetDetectedLight)) true)
  (AI|AIMoveTo self "0, 0, 0" (Game|GetPlayerCharacter 0) 5.0 false))

(event Custom|ReturnToStationaryPoint
  (AI|AIMoveTo self (Transformation|GetActorLocation (Utilities|Array|Get(acopy) (Variables|Default|GetWayPoint))) 0 5.0 false
    (:OnSuccess
      (CallFunction|Looking))))

(event EventBeginPlay
  (bind _asalert_abp (Utilities|Casting|CastToAlert_ABP (Components|SkeletalMesh|GetAnimInstance (Variables|Default|GetAlertMesh))))
  (Variables|Default|SetAlertABP_Ref _asalert_abp)
  (bind _asquestion_mark_abp (Utilities|Casting|CastToQuestionMark_ABP (Components|SkeletalMesh|GetAnimInstance (Variables|Default|GetQuestionMark))))
  (Variables|Default|SetQuestionMarkABP_Ref _asquestion_mark_abp)
  (bind _asguard_abp (Utilities|Casting|CastToGuard_ABP (Components|SkeletalMesh|GetAnimInstance (Variables|Character|GetMesh))))
  (Variables|Default|SetGuardABP_Ref _asguard_abp))

(fn ConstructionScript)

(fn ToggleArrowVisibility
  (bind _arrowmesh (Variables|Default|GetArrowMesh))
  (if (Rendering|IsVisible _arrowmesh)
    (Rendering|SetVisibility _arrowmesh false false)
    (else
      (Rendering|SetVisibility _arrowmesh true false))))

(fn PlayAlertSound
  (Audio|PlaySoundatLocation "/Game/Sound/UI_Animate_Clean_Beeps_Appear_stereo_Cue.UI_Animate_Clean_Beeps_Appear_stereo_Cue" (Transformation|GetWorldLocation (Variables|Default|GetAlertMesh)) "0, 0, 0" 0.5 1.0 0.0 "/Game/Assets/Attenuation/AlertAttenuation.AlertAttenuation" 0 0))

(fn PlayQuestionSound
  (Audio|PlaySoundatLocation "/Game/Sound/UI_Animate_Clean_Beeps_Disappear_stereo_Cue.UI_Animate_Clean_Beeps_Disappear_stereo_Cue" (Transformation|GetWorldLocation (Variables|Default|GetQuestionMark)) "0, 0, 0" 0.5 1.0 0.0 "/Game/Assets/Attenuation/AlertAttenuation.AlertAttenuation" 0 0))