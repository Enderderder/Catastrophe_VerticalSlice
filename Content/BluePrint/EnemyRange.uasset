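; EnemyRange is a ranged enemy that turns toward the player character and shoots projectiles at it.
; When pawn sensing sees a ThirdPersonCharacter, it snaps its rotation to face it.
; It then spawns a FirstPersonProjectile at FirePoint and launches it along the Cube's forward vector with a velocity-change impulse.
; A SpawnBullet flag reset after a delay limits the fire rate.
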(event OnSeePawn(PawnSensing)
  (params (Pawn :type Pawn%20Object%20Reference))
  (bind _asthird_person_character (Utilities|Casting|CastToThirdPersonCharacter Pawn))
  (Utilities|FlowControl|Sequence
    (:then_0
      (Transformation|SetActorRotation (Math|Rotator|FindLookatRotation (Transformation|GetActorLocation) (Transformation|GetActorLocation _asthird_person_character))))
    (:then_1
      (if (Variables|Default|GetSpawnBullet)
        (bind _returnvalue (Game|SpawnActorfromClass "/Game/BluePrint/FirstPersonProjectile.FirstPersonProjectile_C" (Transformation|GetWorldTransform (Variables|Default|GetFirePoint)) "Undefined" 0 0))
        (Physics|AddImpulse (Variables|/Game/BluePrint/FirstPersonProjectile.FirstPersonProjectile_C|GetSphere _returnvalue) (* (Math|Vector|GetForwardVector (Variables|Default|GetCube)) (Variables|Default|GetBulletSpeed)) "None" true)
        (Variables|Default|SetSpawnBullet false)
        (Utilities|FlowControl|Delay 1.5)
        (Variables|Default|SetSpawnBullet true)))))

(fn ConstructionScript)