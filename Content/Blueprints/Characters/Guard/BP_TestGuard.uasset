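; Test guard character that extends a parent guard's state machine and sends a caught player to the HoldingCell level through the respawn subsystem.
; While sleeping, Tick checks a placeholder hearing sphere for a moving, non-crouched player, then enters wake-up stage one with a look-around montage.
; A timer returns it to sleep unless a state change clears it.
; Alert and question-mark indicators suppress each other via their AnimInstances, and stun activates a particle.
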(event OnComponentBeginOverlap(CatchHitBox)
  (params (OverlappedComponent :type Primitive%20Component%20Object%20Reference) (OtherActor :type Actor%20Object%20Reference) (OtherComp :type Primitive%20Component%20Object%20Reference) (OtherBodyIndex :type Integer) (bFromSweep :type Boolean) (SweepResult :type Hit%20Result%20Structure%20%28by%20ref%29))
  (bind _returnvalue (Subsystems|GetRespawnSubsystem))
  (if (Actor|ActorHasTag OtherActor "Player")
    (bind _returnvalue_2 (Game|GetCurrentLevelName true))
    (Class|RespawnSubsystem|LoadLevelStreaming _returnvalue (Utilities|Struct|MakeLoadStreamingLevelInfo (Utilities|String|StringToName _returnvalue_2) "HoldingCell"))
    (Class|RespawnSubsystem|RespawnPlayeratLocation _returnvalue "HOLDINGCELL")))

(event OnComponentBeginOverlap(StupidFakeBsHearingSphere)
  (params (OverlappedComponent :type Primitive%20Component%20Object%20Reference) (OtherActor :type Actor%20Object%20Reference) (OtherComp :type Primitive%20Component%20Object%20Reference) (OtherBodyIndex :type Integer) (bFromSweep :type Boolean) (SweepResult :type Hit%20Result%20Structure%20%28by%20ref%29))
  (if (Actor|ActorHasTag OtherActor "Player")
    (Variables|Default|SetbPlayerInSleepDetectRange true)))

(event OnComponentEndOverlap(StupidFakeBsHearingSphere)
  (params (OverlappedComponent :type Primitive%20Component%20Object%20Reference) (OtherActor :type Actor%20Object%20Reference) (OtherComp :type Primitive%20Component%20Object%20Reference) (OtherBodyIndex :type Integer))
  (if (Actor|ActorHasTag OtherActor "Player")
    (Variables|Default|SetbPlayerInSleepDetectRange false)))

(event Event_OnStunBegin
  (Components|Activation|Activate (Variables|Default|GetStunParticle) true))

(event EventTick
  (params (DeltaSeconds :type Float%20%28single-precision%29))
  ;[1 1 1] Testing Shit
  (switch Utilities|FlowControl|Switch|SwitchonEGuardState (Variables|Default|GetGuardState)
    (:SLEEPING
      (if (Variables|Default|GetbPlayerInSleepDetectRange)
        (bind _playerref (Variables|Default|GetPlayerRef)
          (:then
            (if (and (Math|Vector|NotEqual(Vector) (Transformation|GetVelocity _playerref) "0, 0, 0" 0.0001) (not (AI|Components|NavMovement|IsCrouching (Variables|/Script/Engine.Character|GetCharacterMovement _playerref))))
              (Class|Guard|SetGuardState "WAKEUP_STAGEONE")
              (CallFunction|LookAround)))
          (:else))))))

(event EventOnGuardStateChange
  (params (_oldState :type EGuardState%20Enum :default "STATIONARY") (_newState :type EGuardState%20Enum :default "STATIONARY"))
  (|CallParentFunction _oldState _newState)
  (|SwitchForOldState _oldState)
  (|SwitchForNewState _newState))

(event EventToggleQuestionIndicator
  (params (_b :type Boolean))
  (bind _abp_questionmark (Utilities|GetQuestionMarkAnimInstance)
    (:Success
      (bind _output_get (Variables|/Game/Assets/Questionmark/ABP_QuestionMark.ABP_QuestionMark_C|SetbQuestioning _abp_questionmark _b))
      (if _output_get
        (bind _abp_alert (Utilities|GetAlertAnimInstance)
          (:Success
            (Variables|/Game/Assets/Alert/ABP_Alert.ABP_Alert_C|SetbAlerted _abp_alert false)))))))

(event EventToggleAlertIndicator
  (params (_b :type Boolean))
  (bind _abp_alert (Utilities|GetAlertAnimInstance)
    (:Success
      (bind _output_get (Variables|/Game/Assets/Alert/ABP_Alert.ABP_Alert_C|SetbAlerted _abp_alert _b))
      (if _output_get
        (bind _abp_questionmark (Utilities|GetQuestionMarkAnimInstance)
          (:Success
            (Variables|/Game/Assets/Questionmark/ABP_QuestionMark.ABP_QuestionMark_C|SetbQuestioning _abp_questionmark false)))))))

(fn ConstructionScript)

(fn GetPerceptionLocRot
  (bind _returnvalue (Utilities|Name|MakeLiteralName "PerceptionSocket"))
  (bind _mesh (Variables|Character|GetMesh))
  (bind _returnvalue_2 (Transformation|GetSocketTransform _mesh _returnvalue "RTS_World"))
  (return (.location _returnvalue_2) (.rotation _returnvalue_2)))

(fn LookAround
  (bind _guardaniminstance (Variables|Default|GetGuardAnimInstance)
    (:then
      (bind _returnvalue (Animation|Montage|MontagePlay _guardaniminstance "/Game/Assets/GuardAssets/Animations/AM_Guard_Look.AM_Guard_Look" 1.0 "MontageLength" 0.0 true))
      (return _returnvalue))
    (:else
      (return 0.0))))

(event Custom|ReturnToSleep
  (Class|Guard|SetGuardState "SLEEPING"))