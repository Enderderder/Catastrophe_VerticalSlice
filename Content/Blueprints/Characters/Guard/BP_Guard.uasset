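; BP_Guard is the guard character, providing its perception point, look-around animation and overhead state indicators.
; Question-mark and alert toggles drive the anim instances of their mark meshes, and turning one on switches the other off.
; A player overlapping the Sound component sets the guard to the investigating state.
; Perception location and rotation come from a mesh socket, and LookAround plays a montage and returns its duration.
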(event OnComponentBeginOverlap(Sound)
  (params (OverlappedComponent :type Primitive%20Component%20Object%20Reference) (OtherActor :type Actor%20Object%20Reference) (OtherComp :type Primitive%20Component%20Object%20Reference) (OtherBodyIndex :type Integer) (bFromSweep :type Boolean) (SweepResult :type Hit%20Result%20Structure%20%28by%20ref%29))
  (Utilities|Casting|CastToPlayerCharacter OtherActor)
  (Class|Guard|SetGuardState "INVESTATING"))

(event EventToggleQuestionIndicator
  (params (_b :type Boolean))
  (bind _abp_questionmark (Utilities|GetQuestionMarkAnimInstance)
    (:Success
      (bind _output_get (Variables|/Game/Assets/Questionmark/ABP_QuestionMark.ABP_QuestionMark_C|SetbQuestioning _abp_questionmark _b))
      (if _output_get
        (bind _abp_alert (Utilities|GetAlertAnimInstance)
          (:Success
            (Variables|/Game/Assets/Alert/ABP_Alert.ABP_Alert_C|SetbAlerted _abp_alert false)))))))

(event EventToggleAlertIndicator
  (params (_b :type Boolean))
  (bind _abp_alert (Utilities|GetAlertAnimInstance)
    (:Success
      (bind _output_get (Variables|/Game/Assets/Alert/ABP_Alert.ABP_Alert_C|SetbAlerted _abp_alert _b))
      (if _output_get
        (bind _abp_questionmark (Utilities|GetQuestionMarkAnimInstance)
          (:Success
            (Variables|/Game/Assets/Questionmark/ABP_QuestionMark.ABP_QuestionMark_C|SetbQuestioning _abp_questionmark false)))))))

(fn ConstructionScript)

(fn GetPerceptionLocRot
  (bind _returnvalue (Utilities|Name|MakeLiteralName "PerceptionSocket"))
  (bind _mesh (Variables|Character|GetMesh))
  (bind _returnvalue_2 (Transformation|GetSocketTransform _mesh _returnvalue "RTS_World"))
  (return (.location _returnvalue_2) (.rotation _returnvalue_2)))

(fn LookAround
  (bind _returnvalue (Animation|Montage|MontagePlay (Variables|Default|GetGuardAnimInstance) "/Game/Assets/GuardAssets/Animations/AM_Guard_Look.AM_Guard_Look" 1.0 "Duration" 0.0 true))
  (return _returnvalue))