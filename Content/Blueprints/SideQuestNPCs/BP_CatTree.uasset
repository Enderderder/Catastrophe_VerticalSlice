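; Side quest NPC for a cat in a tree, whose branch the player must break in exchange for fish bones.
; Finishing the first dialogue arms the tomato collision, whose overlap briefly simulates physics to drop branch and cat, then re-enables dialogue.
; Completing the follow-up dialogue awards the fish bones.
; Dialogue events update the widget's text and speaker icons, toggle the player HUD, and disable dialogue when the player leaves the trigger.
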(event OnComponentEndOverlap(TriggerBox)
  (params (OverlappedComponent :type Primitive%20Component%20Object%20Reference) (OtherActor :type Actor%20Object%20Reference) (OtherComp :type Primitive%20Component%20Object%20Reference) (OtherBodyIndex :type Integer))
  ;[1 1 1] Walk out range
  (if (Actor|ActorHasTag OtherActor "Player")
    (Class|NPC|DisableDialogue)))

(event OnComponentBeginOverlap(TomatoCollision)
  (params (OverlappedComponent :type Primitive%20Component%20Object%20Reference) (OtherActor :type Actor%20Object%20Reference) (OtherComp :type Primitive%20Component%20Object%20Reference) (OtherBodyIndex :type Integer) (bFromSweep :type Boolean) (SweepResult :type Hit%20Result%20Structure%20%28by%20ref%29))
  (bind _treecat (Variables|Default|GetTreeCat))
  ;[1 1 1] Quest Objective
  (if (Variables|Default|GetCanBreakBranch)
    (Physics|SetSimulatePhysics (Variables|Default|GetBranch) true)
    (Physics|SetSimulatePhysics _treecat true)
    (Utilities|FlowControl|Delay 0.8)
    (Physics|SetSimulatePhysics (Variables|Default|GetBranch) false)
    (Physics|SetSimulatePhysics _treecat false)
    (Variables|Default|SetIsBranchBroken true)
    (Variables|Default|SetCanNPCTalk true)
    (Components|Animation|SetAnimation (Variables|Default|GetTreeCat) "/Game/Assets/Catchild/Animations/A_CatChild_Idle2.A_CatChild_Idle2")))

(event Event_DisableDialogue
  (Widget|SetVisibility (Variables|/Script/Catastrophe_VS.PlayerCharacter|GetPlayerWidget (Variables|Default|GetPlayer)) "Visible"))

(event Event_FinishOldQuest
  ;[1 1 1] Starting Quest
  (Variables|Default|SetCanBreakBranch true)
  (Variables|Default|SetCanNPCTalk false)
  (Components|DestroyComponent (Variables|Default|GetQuestAvailableMesh)))

(event Event_FinishNewQuest
  ;[1 1 1] After completion dialogue
  (Variables|/Script/Catastrophe_VS.PlayerCharacter|SetFishBonesAmount (Variables|Default|GetPlayer) (+ 10 (Variables|/Script/Catastrophe_VS.PlayerCharacter|GetFishBonesAmount (Variables|Default|GetPlayer)))))

(event Event_UpdateWidget
  (bind _dialoguewidget (Variables|Default|GetDialogueWidget))
  ;[1 1 1] Updating Dialogue Widget
  (bind _aswbp_dialogue (Utilities|Casting|CastToWBP_Dialogue (Variables|Default|GetDialogueWidget)))
  (Rendering|Components|TextRender|SetText (Variables|/Game/Assets/UI/Widgets/Dialogue/WBP_Dialogue.WBP_Dialogue_C|GetNPC_Text _aswbp_dialogue) (Utilities|Text|ToText(String) (Variables|Default|GetCurrentNPCDialogueText)))
  (Rendering|Components|TextRender|SetText (Variables|/Game/Assets/UI/Widgets/Dialogue/WBP_Dialogue.WBP_Dialogue_C|GetPlayer_Text _aswbp_dialogue) (Utilities|Text|ToText(String) (Variables|Default|GetCurrentPlayerDialogueText)))
  (bind _aswbp_dialogue_2 (Utilities|Casting|CastToWBP_Dialogue (Variables|Default|GetDialogueWidget)))
  (Class|Image|SetBrush (Variables|/Game/Assets/UI/Widgets/Dialogue/WBP_Dialogue.WBP_Dialogue_C|GetNPC_Icon _aswbp_dialogue_2) (Utilities|Struct|MakeSlateBrush (Class|Widget|GetDesiredSize (Variables|/Game/Assets/UI/Widgets/Dialogue/WBP_Dialogue.WBP_Dialogue_C|GetNPC_Icon _aswbp_dialogue_2)) "(Left=0.000000,Top=0.000000,Right=0.000000,Bottom=0.000000)" "(SpecifiedColor=(R=1.000000,G=1.000000,B=1.000000,A=1.000000),ColorUseRule=UseColor_Specified)" (Variables|Default|GetNPCIcon) "Image" "NoTile" "NoMirror"))
  (if (Variables|Default|GetIsNPCTalking)
    (bind _aswbp_dialogue_3 (Utilities|Casting|CastToWBP_Dialogue _dialoguewidget))
    (Widget|SetVisibility (Variables|/Game/Assets/UI/Widgets/Dialogue/WBP_Dialogue.WBP_Dialogue_C|GetNPC_Icon _aswbp_dialogue_3) "Visible")
    (Widget|SetVisibility (Variables|/Game/Assets/UI/Widgets/Dialogue/WBP_Dialogue.WBP_Dialogue_C|GetPlayer_Icon _aswbp_dialogue_3) "Hidden")
    (else
      (bind _aswbp_dialogue_4 (Utilities|Casting|CastToWBP_Dialogue _dialoguewidget))
      (Widget|SetVisibility (Variables|/Game/Assets/UI/Widgets/Dialogue/WBP_Dialogue.WBP_Dialogue_C|GetNPC_Icon _aswbp_dialogue_4) "Hidden")
      (Widget|SetVisibility (Variables|/Game/Assets/UI/Widgets/Dialogue/WBP_Dialogue.WBP_Dialogue_C|GetPlayer_Icon _aswbp_dialogue_4) "Visible"))))

(event EventBeginPlay
  ;[1 1 1] IDK
  (bind _asplayer_character (Utilities|Casting|CastToPlayerCharacter (Game|GetPlayerCharacter 0)))
  (Variables|Default|SetPlayer _asplayer_character))

(event Event_Interact
  (Widget|SetVisibility (Variables|/Script/Catastrophe_VS.PlayerCharacter|GetPlayerWidget (Variables|Default|GetPlayer)) "Hidden"))

(fn ConstructionScript)