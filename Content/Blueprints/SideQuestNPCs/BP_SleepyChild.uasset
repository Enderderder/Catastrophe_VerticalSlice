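; Side-quest NPC Blueprint for a sleepy child whose lost teddy the player retrieves for a fish-bone reward.
; Finishing the first dialogue disables talking and reveals the teddy with its trigger, registered with the InteractableComponent.
; Interacting inside that trigger removes the teddy and re-enables talking, and the final dialogue awards the fish bones.
; It also fills the dialogue widget, toggling speaker icons, and closes dialogue when the player leaves range.
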(event OnComponentEndOverlap(TriggerBox)
  (params (OverlappedComponent :type Primitive%20Component%20Object%20Reference) (OtherActor :type Actor%20Object%20Reference) (OtherComp :type Primitive%20Component%20Object%20Reference) (OtherBodyIndex :type Integer))
  ;[1 1 1] Walk out range
  (if (Actor|ActorHasTag OtherActor "Player")
    (Class|NPC|DisableDialogue)))

(event OnComponentBeginOverlap(TeddyTrigger)
  (params (OverlappedComponent :type Primitive%20Component%20Object%20Reference) (OtherActor :type Actor%20Object%20Reference) (OtherComp :type Primitive%20Component%20Object%20Reference) (OtherBodyIndex :type Integer) (bFromSweep :type Boolean) (SweepResult :type Hit%20Result%20Structure%20%28by%20ref%29))
  (Utilities|Casting|CastToPlayerCharacter OtherActor)
  (Variables|Default|SetCanPickupTeddy true))

(event OnInteract(InteractableComponent)
  (params (_playerCharacter :type Player%20Character%20Object%20Reference))
  ;[1 1 1] Quest Objective
  (if (Variables|Default|GetCanPickupTeddy)
    (Components|DestroyComponent (Variables|Default|GetTeddyTrigger))
    (Components|DestroyComponent (Variables|Default|GetTeddy))
    (Variables|Default|SetCanNPCTalk true)))

(event OnComponentEndOverlap(TeddyTrigger)
  (params (OverlappedComponent :type Primitive%20Component%20Object%20Reference) (OtherActor :type Actor%20Object%20Reference) (OtherComp :type Primitive%20Component%20Object%20Reference) (OtherBodyIndex :type Integer))
  (Utilities|Casting|CastToPlayerCharacter OtherActor)
  (Variables|Default|SetCanPickupTeddy false))

(event Event_FinishOldQuest
  ;[1 1 1] After starting dialogue
  (Variables|Default|SetCanNPCTalk false)
  (Components|DestroyComponent (Variables|Default|GetQuestAvailableMesh))
  (Collision|SetCollisionEnabled (Variables|Default|GetTeddyTrigger) "QueryAndPhysics")
  (Rendering|SetVisibility (Variables|Default|GetTeddy) true false))

(event Event_FinishNewQuest
  ;[1 1 1] After Finishing dialogue
  (Variables|/Script/Catastrophe_VS.PlayerCharacter|SetFishBonesAmount (Variables|Default|GetPlayer) (+ 20 (Variables|/Script/Catastrophe_VS.PlayerCharacter|GetFishBonesAmount (Variables|Default|GetPlayer)))))

(event Event_UpdateWidget
  (bind _dialoguewidget (Variables|Default|GetDialogueWidget))
  ;[1 1 1] Updating Dialogue Widget
  (bind _aswbp_dialogue (Utilities|Casting|CastToWBP_Dialogue (Variables|Default|GetDialogueWidget)))
  (Rendering|Components|TextRender|SetText (Variables|/Game/Assets/UI/Widgets/Dialogue/WBP_Dialogue.WBP_Dialogue_C|GetNPC_Text _aswbp_dialogue) (Utilities|Text|ToText(String) (Variables|Default|GetCurrentNPCDialogueText)))
  (Rendering|Components|TextRender|SetText (Variables|/Game/Assets/UI/Widgets/Dialogue/WBP_Dialogue.WBP_Dialogue_C|GetPlayer_Text _aswbp_dialogue) (Utilities|Text|ToText(String) (Variables|Default|GetCurrentPlayerDialogueText)))
  (bind _aswbp_dialogue_2 (Utilities|Casting|CastToWBP_Dialogue (Variables|Default|GetDialogueWidget)))
  (Class|Image|SetBrush (Variables|/Game/Assets/UI/Widgets/Dialogue/WBP_Dialogue.WBP_Dialogue_C|GetNPC_Icon _aswbp_dialogue_2) (Utilities|Struct|MakeSlateBrush (Class|Widget|GetDesiredSize (Variables|/Game/Assets/UI/Widgets/Dialogue/WBP_Dialogue.WBP_Dialogue_C|GetNPC_Icon _aswbp_dialogue_2)) "(Left=0.000000,Top=0.000000,Right=0.000000,Bottom=0.000000)" "(SpecifiedColor=(R=1.000000,G=1.000000,B=1.000000,A=1.000000),ColorUseRule=UseColor_Specified)" (Variables|Default|GetNPCIcon) "Image" "NoTile" "NoMirror"))
  (if (Variables|Default|GetIsNPCTalking)
    (bind _aswbp_dialogue_3 (Utilities|Casting|CastToWBP_Dialogue _dialoguewidget))
    (Widget|SetVisibility (Variables|/Game/Assets/UI/Widgets/Dialogue/WBP_Dialogue.WBP_Dialogue_C|GetNPC_Icon _aswbp_dialogue_3) "Visible")
    (Widget|SetVisibility (Variables|/Game/Assets/UI/Widgets/Dialogue/WBP_Dialogue.WBP_Dialogue_C|GetPlayer_Icon _aswbp_dialogue_3) "Hidden")
    (else
      (bind _aswbp_dialogue_4 (Utilities|Casting|CastToWBP_Dialogue _dialoguewidget))
      (Widget|SetVisibility (Variables|/Game/Assets/UI/Widgets/Dialogue/WBP_Dialogue.WBP_Dialogue_C|GetNPC_Icon _aswbp_dialogue_4) "Hidden")
      (Widget|SetVisibility (Variables|/Game/Assets/UI/Widgets/Dialogue/WBP_Dialogue.WBP_Dialogue_C|GetPlayer_Icon _aswbp_dialogue_4) "Visible"))))

(event EventBeginPlay
  ;[1 1 1] IDK
  (bind _asplayer_character (Utilities|Casting|CastToPlayerCharacter (Game|GetPlayerCharacter 0)))
  (Variables|Default|SetPlayer _asplayer_character))

(fn ConstructionScript
  (Class|InteractableComponent|RegisterTriggerVolume (Variables|Default|GetInteractableComponent) (Variables|Default|GetTeddyTrigger)))