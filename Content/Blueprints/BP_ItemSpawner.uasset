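; BP_ItemSpawner is an actor that spawns a single item at a randomly chosen spawn point when play begins.
; On BeginPlay it picks a random index into its SpawnPoints array, treats that entry as a world-axis offset from the root's location, and spawns the Item class there unrotated.
; The spawned actor is stored in SpawnedItem.
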(event EventBeginPlay
  (bind _output_get (Variables|Default|SetRandomNum (Math|Random|RandomIntegerinRange 0 (- (Utilities|Array|Length (Variables|Default|GetSpawnPoints)) 1))))
  (bind _returnvalue (Game|SpawnActorfromClass (Variables|Default|GetItem) (Math|Transform|MakeTransform (+ (Utilities|Array|Get(acopy) (Variables|Default|GetSpawnPoints) _output_get) (Transformation|GetWorldLocation (Variables|Default|GetDefaultSceneRoot))) "0, 0, 0" "1,1,1.000000") "Undefined" 0 0))
  (Variables|Default|SetSpawnedItem _returnvalue))

(fn ConstructionScript)