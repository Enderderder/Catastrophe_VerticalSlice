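; BP_TomatoBad is a thrown physics projectile, launched along its forward vector on BeginPlay through the FishKunai component.
; On hitting anything but the player, it stops, disables physics and plays a splat sound.
; TriggerSphere overlaps open and close the player's interaction, while Tick closes it whenever the player interacts, regardless of overlap.
; The DestroyActor calls are unconnected, so interacting never removes the actor.
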(event OnComponentBeginOverlap(TriggerSphere)
  (params (OverlappedComponent :type Primitive%20Component%20Object%20Reference) (OtherActor :type Actor%20Object%20Reference) (OtherComp :type Primitive%20Component%20Object%20Reference) (OtherBodyIndex :type Integer) (bFromSweep :type Boolean) (SweepResult :type Hit%20Result%20Structure%20%28by%20ref%29))
  (bind _returnvalue (Game|GetPlayerCharacter 0))
  ;[1 1 1] Player Interaction toggle
  (if (== OtherActor _returnvalue)
    (bind _asbp_player_character (Utilities|Casting|CastToBP_PlayerCharacter _returnvalue))
    (Class|PlayerCharacter|OpentoInteraction _asbp_player_character)))

(event OnComponentEndOverlap(TriggerSphere)
  (params (OverlappedComponent :type Primitive%20Component%20Object%20Reference) (OtherActor :type Actor%20Object%20Reference) (OtherComp :type Primitive%20Component%20Object%20Reference) (OtherBodyIndex :type Integer))
  (bind _returnvalue (Game|GetPlayerCharacter 0))
  ;[1 1 1] Player Interaction toggle
  (if (== _returnvalue OtherActor)
    (bind _asbp_player_character (Utilities|Casting|CastToBP_PlayerCharacter _returnvalue))
    (Class|PlayerCharacter|CloseInteraction _asbp_player_character)))

(event OnComponentHit(FishKunai)
  (params (HitComponent :type Primitive%20Component%20Object%20Reference) (OtherActor :type Actor%20Object%20Reference) (OtherComp :type Primitive%20Component%20Object%20Reference) (NormalImpulse :type Vector :default "0, 0, 0") (Hit :type Hit%20Result%20Structure%20%28by%20ref%29))
  (bind _fishkunai (Variables|Default|GetFishKunai))
  (if (!= HitComponent (Game|GetPlayerCharacter 0))
    (Physics|SetPhysicsLinearVelocity _fishkunai "0, 0, 0" false "None")
    (Physics|SetSimulatePhysics _fishkunai false)
    (Audio|PlaySound2D "/Game/Sound/GORE_Splat_Hit_Bubbles_mono_Cue.GORE_Splat_Hit_Bubbles_mono_Cue" 1.0 1.0 0.0 0 0)))

(event EventBeginPlay
  (Physics|AddImpulse (Variables|Default|GetFishKunai) (* (Math|Vector|GetForwardVector (Transformation|GetActorRotation)) (Variables|Default|GetProjectileSpeed)) "None" false))

(event EventTick
  (params (DeltaSeconds :type Float%20%28single-precision%29))
  ;[1 1 1] When player push the interact button
  (bind _asbp_player_character (Utilities|Casting|CastToBP_PlayerCharacter (Game|GetPlayerCharacter 0)))
  (bind _returnvalue (Class|PlayerCharacter|IsPlayerInteracting _asbp_player_character))
  (if _returnvalue
    (Class|PlayerCharacter|CloseInteraction _asbp_player_character)))

(fn ConstructionScript)

(fn ShowTriggerDebugValue
  (bind _triggersphere (Variables|Default|GetTriggerSphere))
  (Class|VisualLoggerKismetLibrary|LogLocation _triggersphere (Transformation|GetWorldLocation _triggersphere) "" "(R=0.000000,G=0.000000,B=1.000000,A=1.000000)" 1e+01 "VisLogBP" true))