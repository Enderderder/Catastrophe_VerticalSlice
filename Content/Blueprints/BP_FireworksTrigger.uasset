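; BP_FireworksTrigger is a trigger actor that reveals fireworks when the player enters it after the item to steal is no longer usable.
; On BeginPlay it hides the particle component of every entry in its Fireworks array.
; Trigger overlaps from BP_PlayerCharacter check ItemToSteal's IsUsable flag and, when false, make those particles visible.
; It only toggles visibility, never activating the particle systems or hiding them again.
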(event OnComponentBeginOverlap(Trigger)
  (params (OverlappedComponent :type Primitive%20Component%20Object%20Reference) (OtherActor :type Actor%20Object%20Reference) (OtherComp :type Primitive%20Component%20Object%20Reference) (OtherBodyIndex :type Integer) (bFromSweep :type Boolean) (SweepResult :type Hit%20Result%20Structure%20%28by%20ref%29))
  (bind _asplayer_character (Utilities|Casting|CastToPlayerCharacter OtherActor))
  (Utilities|Casting|CastToBP_PlayerCharacter _asplayer_character)
  (if (not (Variables|/Game/Blueprints/BP_ItemToSteal.BP_ItemToSteal_C|GetisUsable (Variables|Default|GetItemToSteal)))
    (for _array_element (Variables|Default|GetFireworks)
      (Rendering|SetVisibility (Variables|/Script/Engine.Emitter|GetParticleSystemComponent _array_element) true false))))

(event EventBeginPlay
  (for _array_element (Variables|Default|GetFireworks)
    (Rendering|SetVisibility (Variables|/Script/Engine.Emitter|GetParticleSystemComponent _array_element) false false)))

(event Collision|EventActorBeginOverlap
  (params (OtherActor :type Actor%20Object%20Reference)))

(event EventTick
  (params (DeltaSeconds :type Float%20%28single-precision%29)))

(fn ConstructionScript)