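; Level exit trigger for a heist objective that ends the game in a win once the item to steal is no longer usable.
; On BeginPlay it shows a timer widget and passes it a self reference, while Tick accumulates elapsed time.
; When the player character overlaps the box with that condition met, it shows the win screen once, pauses the game and switches to UI-only mouse input.
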(event OnComponentBeginOverlap(TriggerBox)
  (params (OverlappedComponent :type Primitive%20Component%20Object%20Reference) (OtherActor :type Actor%20Object%20Reference) (OtherComp :type Primitive%20Component%20Object%20Reference) (OtherBodyIndex :type Integer) (bFromSweep :type Boolean) (SweepResult :type Hit%20Result%20Structure%20%28by%20ref%29))
  (bind _returnvalue (Game|GetPlayerController 0))
  (if (== OtherActor (Game|GetPlayerCharacter 0))
    (if (not (Variables|/Game/Blueprints/BP_ItemToSteal.BP_ItemToSteal_C|GetisUsable (Variables|Default|GetItemToSteal)))
      (if (not (Variables|Default|GetbHasWon))
        (bind _returnvalue_2 (UserInterface|CreateWidget "/Game/Blueprints/Widgets/WBP_WinScreen.WBP_WinScreen_C" _returnvalue))
        (bind _output_get (Variables|Default|SetWinScreenWidget _returnvalue_2))
        (UserInterface|Viewport|AddtoViewport _output_get 0)
        (Variables|Default|SetbHasWon true)
        (Game|SetGamePaused true)
        (Input|SetInputModeUIOnly _returnvalue 0 "DoNotLock")
        (Variables|/Script/Engine.PlayerController|SetbShowMouseCursor _returnvalue true)))))

(event EventBeginPlay
  (bind _returnvalue (UserInterface|CreateWidget "/Game/Blueprints/Widgets/WBP_Timer.WBP_Timer_C" (Game|GetPlayerController 0)))
  (bind _output_get (Variables|Default|SetTimerWidget _returnvalue))
  (UserInterface|Viewport|AddtoViewport _output_get 0)
  (bind _aswbp_timer (Utilities|Casting|CastToWBP_Timer (Variables|Default|GetTimerWidget)))
  (Variables|/Game/Blueprints/Widgets/WBP_Timer.WBP_Timer_C|SetTrigger _aswbp_timer self))

(event Collision|EventActorBeginOverlap
  (params (OtherActor :type Actor%20Object%20Reference)))

(event EventTick
  (params (DeltaSeconds :type Float%20%28single-precision%29))
  (Variables|Default|SetTimer (+ DeltaSeconds (Variables|Default|GetTimer))))

(fn ConstructionScript)