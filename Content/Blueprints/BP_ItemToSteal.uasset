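; BP_ItemToSteal is the stealable "catch of the day" objective, which creates the goal widget and switches it to "ESCAPE!" once taken.
; Trigger overlap shows camera-facing interaction text and opens player interaction, which Tick polls while the text is visible.
; Pickup hides the cube, removes the outline, reveals the player's carried fish and lowers their speed.
; A separate E key handler also hides the text and disables the item.
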(event OnComponentBeginOverlap(Trigger)
  (params (OverlappedComponent :type Primitive%20Component%20Object%20Reference) (OtherActor :type Actor%20Object%20Reference) (OtherComp :type Primitive%20Component%20Object%20Reference) (OtherBodyIndex :type Integer) (bFromSweep :type Boolean) (SweepResult :type Hit%20Result%20Structure%20%28by%20ref%29))
  (if (and (== OtherActor (Game|GetPlayerCharacter 0)) (Variables|Default|GetisUsable))
    (Rendering|SetVisibility (Variables|Default|GetInteractionText) true false)
    (Class|PlayerCharacter|OpentoInteraction (Variables|Default|GetPlayerReference))))

(event OnComponentEndOverlap(Trigger)
  (params (OverlappedComponent :type Primitive%20Component%20Object%20Reference) (OtherActor :type Actor%20Object%20Reference) (OtherComp :type Primitive%20Component%20Object%20Reference) (OtherBodyIndex :type Integer))
  (if (== OtherActor (Game|GetPlayerCharacter 0))
    (Rendering|SetVisibility (Variables|Default|GetInteractionText) false false)
    (Class|PlayerCharacter|CloseInteraction (Variables|Default|GetPlayerReference))))

(event EventBeginPlay
  (Rendering|SetVisibility (Variables|Default|GetInteractionText) false false)
  (bind _asbp_player_character (Utilities|Casting|CastToBP_PlayerCharacter (Game|GetPlayerCharacter 0)))
  (Variables|Default|SetPlayerReference _asbp_player_character)
  (bind _returnvalue (UserInterface|CreateWidget "/Game/Blueprints/Widgets/WBP_Goal.WBP_Goal_C" (Game|GetPlayerController 0)))
  (bind _output_get (Variables|Default|SetGoalWidget _returnvalue))
  (UserInterface|Viewport|AddtoViewport _output_get 0)
  (bind _aswbp_goal (Utilities|Casting|CastToWBP_Goal (Variables|Default|GetGoalWidget)))
  (Default|ChangeGoal _aswbp_goal "STEAL THE CATCH OF THE DAY"))

(event Collision|EventActorBeginOverlap
  (params (OtherActor :type Actor%20Object%20Reference)))

(event EventTick
  (params (DeltaSeconds :type Float%20%28single-precision%29))
  (bind _playerreference (Variables|Default|GetPlayerReference))
  (bind _interactiontext (Variables|Default|GetInteractionText))
  (if (Rendering|IsVisible _interactiontext)
    (Transformation|SetWorldRotation (Variables|Default|GetInteractionText) (Math|Rotator|FindLookatRotation (Transformation|GetWorldLocation _interactiontext) (Camera|GetCameraLocation (Variables|/Script/Engine.PlayerController|GetPlayerCameraManager (Game|GetPlayerController 0)))) false false)
    (bind _returnvalue (Class|PlayerCharacter|IsPlayerInteracting _playerreference))
    (if _returnvalue
      (CallFunction|PickUpItem)
      (Class|PlayerCharacter|CloseInteraction _playerreference)
      (Rendering|SetVisibility (Variables|Default|GetInteractionText) false false))))

(event Input|KeyboardEvents|E
  (params (Key :type Key%20Structure))
  (:Pressed
    (if (Variables|Default|GetisUsable)
      (if (Variables|/Script/Engine.SceneComponent|GetbVisible (Variables|Default|GetInteractionText))
        (Rendering|SetVisibility (Variables|Default|GetInteractionText) false false)
        (Variables|Default|SetisUsable false)))))

(fn ConstructionScript)

(fn PickUpItem
  (Rendering|SetVisibility (Variables|Default|GetCube) false false)
  (Variables|Default|SetisUsable false)
  (bind _aswbp_goal (Utilities|Casting|CastToWBP_Goal (Variables|Default|GetGoalWidget)))
  (Default|ChangeGoal _aswbp_goal "ESCAPE!")
  (bind _asbp_player_character (Utilities|Casting|CastToBP_PlayerCharacter (Game|GetPlayerCharacter 0)))
  (Rendering|SetVisibility (Variables|/Script/Prototype_NinjaPuss.PlayerCharacter|GetFishToCarry _asbp_player_character) true false)
  (Components|DestroyComponent (Variables|Default|GetOutline))
  (Default|LowerSpeed _asbp_player_character)
  (Class|PlayerCharacter|GrabbingFish _asbp_player_character))