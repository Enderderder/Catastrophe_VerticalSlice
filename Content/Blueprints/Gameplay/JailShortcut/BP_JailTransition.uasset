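; Jail shortcut actor with rock and pipe interactables that control a transition gated on removing the rock.
; Interacting with the rock sets RockRemoved and plays the S_RockPush level sequence, disabling input and hiding the player until it finishes.
; The pipe then moves the player to RockSpawn, or briefly shows a WBP_CellBlock widget if the rock is still in place.
; The construction script registers trigger volumes and prompt UI; InteractableIntoCell gets only UI.
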(event OnInteract(InteractablePipe)
  (params (_playerCharacter :type Player%20Character%20Object%20Reference))
  (if (Variables|Default|GetbRockRemoved)
    (Transformation|SetActorTransform (Game|GetPlayerCharacter 0) (Math|Conversions|ToTransform(Vector) (Transformation|GetWorldLocation (Variables|Default|GetRockSpawn))))
    (else
      (bind _returnvalue (UserInterface|CreateWidget "/Game/Assets/UI/Widgets/WBP_CellBlock.WBP_CellBlock_C"))
      (bind _output_get (Variables|Default|SetNope%20widget _returnvalue))
      (UserInterface|Viewport|AddtoViewport _output_get 0)
      (Utilities|FlowControl|Delay 3.0)
      (Widget|RemovefromParent (Variables|Default|GetNope%20widget)))))

(event OnInteract(InteractableRock)
  (params (_playerCharacter :type Player%20Character%20Object%20Reference))
  (Variables|Default|SetbRockRemoved true)
  (Input|DisableInput (Game|GetPlayerController 0))
  (Rendering|SetActorHiddenInGame (Game|GetPlayerCharacter 0) true)
  (bind _returnvalue (Sequencer|Player|CreateLevelSequencePlayer "/Game/Sequences/S_RockPush.S_RockPush"))
  (bind _output_get (Variables|Default|SetSecretDoorRemoveSequence _returnvalue))
  (Sequencer|Player|Play _output_get :!class /Script/MovieScene.MovieSceneSequencePlayer)
  (EventDispatchers|BindEventtoOnFinished (Variables|Default|GetSecretDoorRemoveSequence) (delegate Custom|OnRemoveDoorFinished)))

(event Custom|OnRemoveDoorFinished
  (Input|EnableInput (Game|GetPlayerController 0))
  (Rendering|SetActorHiddenInGame (Game|GetPlayerCharacter 0) false))

(fn ConstructionScript
  (|CallParentFunction)
  (Class|InteractableComponent|RegisterTriggerVolume (Variables|Default|GetInteractableRock) (Variables|Default|GetRock))
  (Class|InteractableComponent|RegisterTriggerVolume (Variables|Default|GetInteractablePipe) (Variables|Default|GetCell))
  (Class|InteractableComponent|RegisterUiComponent (Variables|Default|GetInteractableRock) (Variables|Default|GetInteractUIRock))
  (Class|InteractableComponent|RegisterUiComponent (Variables|Default|GetInteractablePipe) (Variables|Default|GetInteractUIPipe))
  (Class|InteractableComponent|RegisterUiComponent (Variables|Default|GetInteractable_IntoCell) (Variables|Default|GetTeleportUI)))