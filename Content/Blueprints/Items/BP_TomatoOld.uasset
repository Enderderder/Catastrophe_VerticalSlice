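; BP_TomatoOld is a physics-driven tomato projectile that splats on impact.
; On BeginPlay it applies a forward impulse to TomatoMesh, scaled by ProjectileSpeed, rather than using a movement component.
; When the mesh hits something, it spawns a short-lived splat decal oriented to the impact normal at the mesh location, plays an attenuated splat sound there and destroys itself.
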(event OnComponentHit(TomatoMesh)
  (params (HitComponent :type Primitive%20Component%20Object%20Reference) (OtherActor :type Actor%20Object%20Reference) (OtherComp :type Primitive%20Component%20Object%20Reference) (NormalImpulse :type Vector :default "0, 0, 0") (Hit :type Hit%20Result%20Structure%20%28by%20ref%29))
  (Rendering|Decal|SpawnDecalatLocation "/Game/Assets/Stall_Fruit/M_TomatoSplat_Decal.M_TomatoSplat_Decal" "50.000000,50.000000,50.000000" (Transformation|GetWorldLocation (Variables|Default|GetTomatoMesh)) (Math|Rotator|MakeRotationfromAxes (.ImpactNormal (Collision|BreakHitResult Hit)) "0, 0, 0" "0, 0, 0") 5.0)
  (Audio|PlaySoundatLocation "/Game/Sound/GORE_Splat_Hit_Bubbles_mono_Cue.GORE_Splat_Hit_Bubbles_mono_Cue" (Transformation|GetWorldLocation (Variables|Default|GetTomatoMesh)) "0, 0, 0" 1.0 1.0 0.0 "/Game/Assets/Attenuation/ATT_Splash.ATT_Splash" 0 0)
  (Actor|DestroyActor))

(event EventBeginPlay
  (Physics|AddImpulse (Variables|Default|GetTomatoMesh) (* (Math|Vector|GetForwardVector (Transformation|GetActorRotation)) (Variables|Default|GetProjectileSpeed)) "None" false))

(fn ConstructionScript)