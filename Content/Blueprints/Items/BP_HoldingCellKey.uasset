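; BP_HoldingCellKey is a holding cell key pickup that completes its quest objective when picked up.
; RecievePickUpItem calls CompleteObjective on the QuestObjective, then destroys the actor.
; The objective's activate and complete events print the task's short description to screen.
; An unconnected chain that would activate the DoorTrigger tagged ExitPrisonLevelTrigger never runs, so the key does not enable that door.
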(event OnObjectiveActivate(QuestObjective)
  ;[1 1 1] Print to screen when QuestObjective is activated/completed
  (Development|PrintString (Utilities|String|Append "New Task: " (Variables|/Script/Catastrophe_VS.QuestObjectiveComponent|GetShortDescription (Variables|Default|GetQuestObjective)))))

(event OnObjectiveComplete(QuestObjective)
  ;[1 1 1] Print to screen when QuestObjective is activated/completed
  (Development|PrintString (Utilities|String|Append "Task Completed: " (Variables|/Script/Catastrophe_VS.QuestObjectiveComponent|GetShortDescription (Variables|Default|GetQuestObjective)))))

(event EventRecievePickUpItem
  (Class|QuestObjectiveComponent|CompleteObjective (Variables|Default|GetQuestObjective))
  (Actor|DestroyActor))

(fn ConstructionScript)