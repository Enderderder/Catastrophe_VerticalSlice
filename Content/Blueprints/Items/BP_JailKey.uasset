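; BP_JailKey is a pickup key item tied to a quest objective.
; Picking it up completes its QuestObjective and destroys the actor.
; When the objective activates, the player's quest widget updates with it.
; Each tick, an objective marker shows only while the objective is active, polled rather than driven by the objective's events.
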(event OnObjectiveActivate(QuestObjective)
  ;[1 1 1] Print to screen when QuestObjective is activated/completed
  (bind _asbp_player_character (Utilities|Casting|CastToBP_PlayerCharacter (Game|GetPlayerCharacter 0)))
  (Default|Update (Variables|/Game/Blueprints/Characters/BP_PlayerCharacter.BP_PlayerCharacter_C|GetQuestWidget _asbp_player_character) (Variables|Default|GetQuestObjective)))

(event OnObjectiveComplete(QuestObjective)
  ;[1 1 1] Print to screen when QuestObjective is activated/completed
)

(event EventTick
  (params (DeltaSeconds :type Float%20%28single-precision%29))
  (bind _objectivemarker (Variables|Default|GetObjectiveMarker))
  (if (Utilities|Enum|Equal(Enum) (Variables|/Script/Catastrophe_VS.QuestObjectiveComponent|GetObjectiveState (Variables|Default|GetQuestObjective)) "Active")
    (Rendering|SetVisibility _objectivemarker true false)
    (else
      (Rendering|SetVisibility _objectivemarker false false))))

(event EventRecievePickUpItem
  (Class|QuestObjectiveComponent|CompleteObjective (Variables|Default|GetQuestObjective))
  (Actor|DestroyActor))

(fn ConstructionScript)