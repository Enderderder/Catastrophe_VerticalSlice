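; Cat tree actor where a cat and its branch can be knocked down after the player interacts with it.
; Overlapping the DialogueBox sets CanTalk, which lets the Interact input permanently arm CanBreakBranch.
; Once armed, any overlap on TomatoCollision briefly simulates physics on the branch and cat, then switches it off after a short delay to halt the fall.
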(event OnComponentBeginOverlap(TomatoCollision)
  (params (OverlappedComponent :type Primitive%20Component%20Object%20Reference) (OtherActor :type Actor%20Object%20Reference) (OtherComp :type Primitive%20Component%20Object%20Reference) (OtherBodyIndex :type Integer) (bFromSweep :type Boolean) (SweepResult :type Hit%20Result%20Structure%20%28by%20ref%29))
  ;[1 1 1] Knocking him out of the tree
  (if (Variables|Default|GetCanBreakBranch)
    (Physics|SetSimulatePhysics (Variables|Default|GetBranch) true)
    (Physics|SetSimulatePhysics (Variables|Default|GetCat) true)
    (Utilities|FlowControl|Delay 0.8)
    (Physics|SetSimulatePhysics (Variables|Default|GetBranch) false)
    (Physics|SetSimulatePhysics (Variables|Default|GetCat) false)))

(event OnComponentBeginOverlap(DialogueBox)
  (params (OverlappedComponent :type Primitive%20Component%20Object%20Reference) (OtherActor :type Actor%20Object%20Reference) (OtherComp :type Primitive%20Component%20Object%20Reference) (OtherBodyIndex :type Integer) (bFromSweep :type Boolean) (SweepResult :type Hit%20Result%20Structure%20%28by%20ref%29))
  ;[1 1 1] Can talk?
  (Variables|Default|SetCanTalk? true))

(event OnComponentEndOverlap(DialogueBox)
  (params (OverlappedComponent :type Primitive%20Component%20Object%20Reference) (OtherActor :type Actor%20Object%20Reference) (OtherComp :type Primitive%20Component%20Object%20Reference) (OtherBodyIndex :type Integer))
  ;[1 1 1] Can talk?
  (Variables|Default|SetCanTalk? false))

(event Input|ActionEvents|InputActionInteract
  (params (Key :type Key%20Structure))
  (:Pressed
    (if (Variables|Default|GetCanTalk?)
      (Variables|Default|SetCanBreakBranch true))))

(fn ConstructionScript)