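; BP_HidingUrn is a single-use interactable urn that hides the player for a limited time, then shatters.
; JumpIn hides the player, disables collision, movement and shooting, teleports them above the urn and shows a timer widget.
; JumpOut, triggered by re-interaction or timeout, restores the player and breaks the destructible mesh with sound.
; A short delay re-registers it as interaction target against double taps, while Tick turns the prompt toward the camera.
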(event EventBeginPlay
  ;[1 1 1] BeginPlay
  (Rendering|SetVisibility (Variables|Default|GetInteractionText) false false))

(event EventTick
  (params (DeltaSeconds :type Float%20%28single-precision%29))
  (bind _interactiontext (Variables|Default|GetInteractionText))
  ;[1 1 1] Interaction text rotation
  (if (Rendering|IsVisible _interactiontext)
    (Transformation|SetWorldRotation (Variables|Default|GetInteractionText) (Math|Rotator|FindLookatRotation (Transformation|GetWorldLocation _interactiontext) (Camera|GetCameraLocation (Variables|/Script/Engine.PlayerController|GetPlayerCameraManager (Game|GetPlayerController 0)))) false false)
    (elif (Variables|Default|GetbPlayerIn)
      (Rendering|SetVisibility (Variables|Default|GetInteractionText) true false))))

(event EventReciveInteractionStart
  ;[1 1 1] Interacting
  (if (not (Variables|Default|GetbHasUsed))
    (if (Variables|Default|GetbPlayerIn)
      (CallFunction|JumpOut)
      (Class|InteractActor|EndInteraction)
      (else
        (CallFunction|Jumpin)
        (bind _returnvalue (Utilities|Time|SetTimerbyFunctionName self "SetSelfToInteractTarget" (Variables|Default|GetDoubleTapSafeDelay)))
        (Variables|Default|SetSpamProtectionTimerHandle _returnvalue)))))

(event EventReciveInteractionEnd
  ;[1 1 1] End Interaction
  (Class|InteractActor|DisableInteractActor)
  (Utilities|Time|ClearandInvalidateTimerbyHandle (Variables|Default|GetSpamProtectionTimerHandle)))

(fn ConstructionScript)

(fn Jumpin
  (bind _returnvalue (Transformation|GetActorLocation))
  (bind _playerreference (Variables|Default|GetPlayerReference))
  (bind _playerreference_2 (Variables|Default|GetPlayerReference))
  (bind (_x _y _z) (Math|Vector|BreakVector _returnvalue))
  (bind _charactermovement (Variables|/Script/Engine.Character|GetCharacterMovement _playerreference_2))
  (Variables|Default|SetbPlayerIn true)
  (Variables|Default|SetWalkSpeed (Variables|/Script/Engine.CharacterMovementComponent|GetMaxWalkSpeed _charactermovement))
  (Variables|/Script/Engine.CharacterMovementComponent|SetMaxWalkSpeed _charactermovement 0.0)
  (Variables|Default|Setplayerlocation (Transformation|GetActorLocation (Variables|Default|GetPlayerReference)))
  (Rendering|SetActorHiddenInGame _playerreference true)
  (Collision|SetCollisionEnabled (Variables|/Script/Engine.Character|GetCapsuleComponent _playerreference) "NoCollision")
  (bind _output_get (Variables|Default|Setendlocation (Math|Vector|MakeVector _x _y (+ _z 2e+02))))
  (Transformation|SetActorLocation (Variables|Default|GetPlayerReference) _output_get false true)
  (Variables|/Script/Catastrophe_VS.PlayerCharacter|SetbAbleToShootTomato (Variables|Default|GetPlayerReference) false)
  (Components|DestroyComponent (Variables|Default|GetOutline))
  (Utilities|Time|SetTimerbyFunctionName self "JumpOut" (Variables|Default|GetJumpOutTime))
  (bind _returnvalue_2 (UserInterface|CreateWidget "/Game/Blueprints/Widgets/WBP_UrnTimer.WBP_UrnTimer_C"))
  (bind _output_get_2 (Variables|Default|SetTimerDestroy _returnvalue_2))
  (UserInterface|Viewport|AddtoViewport _output_get_2 0))

(fn JumpOut
  (bind _playerreference (Variables|Default|GetPlayerReference))
  (bind _urndestructiblemesh (Variables|Default|GetUrnDestructibleMesh))
  (bind _returnvalue (Transformation|GetWorldLocation _urndestructiblemesh))
  (Variables|Default|SetbHasUsed true)
  (Variables|/Script/Engine.CharacterMovementComponent|SetMaxWalkSpeed (Variables|/Script/Engine.Character|GetCharacterMovement (Variables|Default|GetPlayerReference)) (Variables|Default|GetWalkSpeed))
  (Transformation|SetActorLocation _playerreference (Variables|Default|Getplayerlocation) false true)
  (Rendering|SetActorHiddenInGame _playerreference false)
  (Collision|SetCollisionEnabled (Variables|/Script/Engine.Character|GetCapsuleComponent (Variables|Default|GetPlayerReference)) "QueryAndPhysics")
  (Variables|/Script/Catastrophe_VS.PlayerCharacter|SetbAbleToShootTomato (Variables|Default|GetPlayerReference) true)
  (Rendering|SetVisibility (Variables|Default|GetInteractionText) false false)
  (Widget|RemovefromParent (Variables|Default|GetTimerDestroy))
  (Utilities|Time|ClearTimerbyFunctionName self "JumpOut")
  (Class|DestructibleComponent|ApplyDamage _urndestructiblemesh 1.0 _returnvalue _returnvalue 1.0)
  (Components|DestroyComponent (Variables|Default|GetStaticMesh))
  (Audio|PlaySound2D "/Game/Sound/GLASS_Fragment_03_mono_Cue.GLASS_Fragment_03_mono_Cue" 1.0 1.0 0.0 0 0))

(fn SetSelftoInteractTarget
  (Class|PlayerCharacter|SetInteractionTarget (Variables|Default|GetPlayerReference) self))