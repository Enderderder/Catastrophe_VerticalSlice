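; BP_NPC_Prisoner is an interactable prisoner NPC that shows a jail dialogue widget and advances a quest objective.
; On interact, it hides its text render and displays WBP_JailNPC on screen for a few seconds.
; It then removes the widget, wipes all saved games through the save subsystem, creates and loads a fresh slot 0 save, and calls CompleteObjective on its QuestObjective.
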(event EventBeginPlay)

(event Collision|EventActorBeginOverlap
  (params (OtherActor :type Actor%20Object%20Reference)))

(event EventTick
  (params (DeltaSeconds :type Float%20%28single-precision%29)))

(event Event_Interact
  (bind _returnvalue (Subsystems|GetSaveGameSubsystem))
  (Rendering|SetVisibility (Variables|Default|GetTextRender) false false)
  (bind _returnvalue_2 (UserInterface|CreateWidget "/Game/Blueprints/Widgets/Dialogue/WBP_JailNPC.WBP_JailNPC_C"))
  (bind _output_get (Variables|Default|Setwig _returnvalue_2))
  (UserInterface|Viewport|AddtoViewport _output_get 0)
  (Utilities|FlowControl|Delay 5.0)
  (Widget|RemovefromParent (Variables|Default|Getwig))
  (Class|SaveGameSubsystem|DeleteAllSavedGame _returnvalue)
  (Class|SaveGameSubsystem|CreateSavedGame _returnvalue)
  (Class|SaveGameSubsystem|LoadSavedGame _returnvalue)
  (Class|QuestObjectiveComponent|CompleteObjective (Variables|Default|GetQuestObjective)))

(fn ConstructionScript)