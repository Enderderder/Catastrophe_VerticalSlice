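; BP_ClimbableStallReverse is a climbable stall, named as a reverse variant, that changes appearance as it is used.
; On BeginPlay it rebuilds WayPointArray from three waypoints that define the climbing route.
; Interaction start destroys the Outline component and reveals the Ripped component, and interaction end destroys ClimbMesh.
; The climb movement itself is not implemented in this graph.
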(event EventBeginPlay
  (bind _waypointarray (Variables|Default|GetWayPointArray))
  ;[1 1 1] Setup the array of way point  for climbing
  (Utilities|Array|Clear _waypointarray)
  (Utilities|Array|AppendArray _waypointarray (Utilities|Array|MakeArray (Variables|Default|GetWayPoint_1) (Variables|Default|GetWayPoint_2) (Variables|Default|GetWayPoint_3))))

(event Collision|EventActorBeginOverlap
  (params (OtherActor :type Actor%20Object%20Reference)))

(event EventTick
  (params (DeltaSeconds :type Float%20%28single-precision%29)))

(event EventReciveInteractionStart
  ;[1 1 1] OnUse
  (Components|DestroyComponent (Variables|Default|GetOutline))
  (Rendering|SetVisibility (Variables|Default|GetRipped) true false))

(event EventReciveInteractionEnd
  ;[1 1 1] OnUse
  (Components|DestroyComponent (Variables|Default|GetClimbMesh)))

(fn ConstructionScript)