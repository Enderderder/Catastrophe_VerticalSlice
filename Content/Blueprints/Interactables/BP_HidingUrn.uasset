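; BP_HidingUrn is an interactable urn the player jumps into, with a countdown timer shown on a widget component.
; Jumping in shows the WBP_UrnTimer widget, resets it and starts its countdown.
; Jumping out hides the widget and plays a glass fragment sound.
; Each tick rotates the widget to face the player's follow camera, billboard style.
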(event EventTick
  (params (DeltaSeconds :type Float%20%28single-precision%29))
  (bind _asbp_player_character (Utilities|Casting|CastToBP_PlayerCharacter (Game|GetPlayerCharacter 0)))
  (Transformation|SetWorldRotation (Variables|Default|GetWidget) (Math|Rotator|FindLookatRotation (Transformation|GetWorldLocation (Variables|Default|GetWidget)) (Transformation|GetWorldLocation (Variables|/Script/Catastrophe_VS.PlayerCharacter|GetFollowCamera _asbp_player_character))) false false))

(event Event_JumpIn
  (params (_playerCharacter :type Player%20Character%20Object%20Reference))
  (bind _widget (Variables|Default|GetWidget))
  (bind _returnvalue (UserInterface|GetUserWidgetObject _widget))
  (bind _aswbp_urn_timer (Utilities|Casting|CastToWBP_UrnTimer _returnvalue))
  ;[1 1 1] On Jump In Urn
  (Rendering|SetVisibility _widget true false)
  (Default|ResetTimer _aswbp_urn_timer)
  (Variables|/Game/Assets/UI/Widgets/WBP_UrnTimer.WBP_UrnTimer_C|SetbIsCountingDown _aswbp_urn_timer true))

(event Event_JumpOut
  (params (_playerCharacter :type Player%20Character%20Object%20Reference))
  ;[1 1 1] On Jump Out of Urn
  (Rendering|SetVisibility (Variables|Default|GetWidget) false false)
  (Audio|PlaySound2D "/Game/Sound/GLASS_Fragment_03_mono_Cue.GLASS_Fragment_03_mono_Cue" 1.0 1.0 0.0 0 0))

(fn ConstructionScript)