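; BP_StackedCrates is an interactable stack of crates that falls over and then acts as an obstacle.
; On BeginPlay it caches the CratesMesh anim instance as ABP_StackedCrates and disables BlockVolume collision.
; The _PlayCrateAnim event sets the Fallen flag on the anim blueprint, then after a short delay enables query and physics collision on BlockVolume.
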(event Event_PlayCrateAnim
  ;[1 1 1] Crate Fallen Anim
  (Variables|/Game/Assets/StackedCrates/ABP_StackedCrates.ABP_StackedCrates_C|SetbFallen (Variables|Default|GetAnimInstance) true)
  (Utilities|FlowControl|Delay 0.4)
  (Collision|SetCollisionEnabled (Variables|Default|GetBlockVolume) "QueryAndPhysics"))

(event EventBeginPlay
  ;[1 1 1] Begin Play
  (bind _asabp_stacked_crates (Utilities|Casting|CastToABP_StackedCrates (Components|SkeletalMesh|GetAnimInstance (Variables|Default|GetCratesMesh))))
  (Variables|Default|SetAnimInstance _asabp_stacked_crates)
  (Collision|SetCollisionEnabled (Variables|Default|GetBlockVolume) "NoCollision"))

(fn ConstructionScript)