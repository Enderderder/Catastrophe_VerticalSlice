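; Shop NPC interactable that puts the player into and out of a shop interface mode.
; On BeginPlay it passes WBP_Shop to WidgetInit to set up the shop widget.
; Enabling the shop switches to UI-only input, shows the cursor and disables character movement.
; Disabling it restores game input and hides the cursor, but does not re-enable movement here.
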(event Event_EnableShop
  (bind _returnvalue (Game|GetPlayerController 0))
  (Input|SetInputModeUIOnly _returnvalue 0 "DoNotLock")
  (Variables|/Script/Engine.PlayerController|SetbShowMouseCursor _returnvalue true)
  (Pawn|Components|CharacterMovement|DisableMovement (Variables|/Script/Engine.Character|GetCharacterMovement (Game|GetPlayerCharacter 0))))

(event Event_DisableShop
  (bind _returnvalue (Game|GetPlayerController 0))
  (Input|SetInputModeGameOnly _returnvalue)
  (Variables|/Script/Engine.PlayerController|SetbShowMouseCursor _returnvalue false))

(event EventBeginPlay
  (Class|Shop|WidgetInit "/Game/Assets/UI/Widgets/WBP_Shop.WBP_Shop_C"))

(fn ConstructionScript)