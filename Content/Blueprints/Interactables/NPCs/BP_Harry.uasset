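; BP_Harry is an NPC interactable that talks with the player through a dialogue widget and pays out fishbones for quests.
; BeginPlay assigns quest objectives to its first three conversations by index.
; Widget updates set both speakers' text and show only the active speaker's icon.
; Leaving the trigger box disables dialogue, and finishing a quest adds the current reward to the player's fishbone count.
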(event OnComponentEndOverlap(TriggerBox)
  (params (OverlappedComponent :type Primitive%20Component%20Object%20Reference) (OtherActor :type Actor%20Object%20Reference) (OtherComp :type Primitive%20Component%20Object%20Reference) (OtherBodyIndex :type Integer))
  ;[1 1 1] Stops dialogue when player walks away
  (Utilities|Casting|CastToBP_PlayerCharacter OtherActor)
  (Class|NPC|DisableDialogue))

(event Event_UpdateWidget
  (bind _dialoguewidget (Variables|Default|GetDialogueWidget))
  (bind _aswbp_dialogue (Utilities|Casting|CastToWBP_Dialogue (Variables|Default|GetDialogueWidget)))
  (Rendering|Components|TextRender|SetText (Variables|/Game/Assets/UI/Widgets/Dialogue/WBP_Dialogue.WBP_Dialogue_C|GetNPC_Text _aswbp_dialogue) (Utilities|Text|ToText(String) (Variables|Default|GetCurrentNPCDialogueText)))
  (Rendering|Components|TextRender|SetText (Variables|/Game/Assets/UI/Widgets/Dialogue/WBP_Dialogue.WBP_Dialogue_C|GetPlayer_Text _aswbp_dialogue) (Utilities|Text|ToText(String) (Variables|Default|GetCurrentPlayerDialogueText)))
  (bind _aswbp_dialogue_2 (Utilities|Casting|CastToWBP_Dialogue (Variables|Default|GetDialogueWidget)))
  (Class|Image|SetBrush (Variables|/Game/Assets/UI/Widgets/Dialogue/WBP_Dialogue.WBP_Dialogue_C|GetNPC_Icon _aswbp_dialogue_2) (Utilities|Struct|MakeSlateBrush (Class|Widget|GetDesiredSize (Variables|/Game/Assets/UI/Widgets/Dialogue/WBP_Dialogue.WBP_Dialogue_C|GetNPC_Icon _aswbp_dialogue_2)) "(Left=0.000000,Top=0.000000,Right=0.000000,Bottom=0.000000)" "(SpecifiedColor=(R=1.000000,G=1.000000,B=1.000000,A=1.000000),ColorUseRule=UseColor_Specified)" (Variables|Default|GetNPCIcon) "Image" "NoTile" "NoMirror"))
  (if (Variables|Default|GetIsNPCTalking)
    (bind _aswbp_dialogue_3 (Utilities|Casting|CastToWBP_Dialogue _dialoguewidget))
    (Widget|SetVisibility (Variables|/Game/Assets/UI/Widgets/Dialogue/WBP_Dialogue.WBP_Dialogue_C|GetNPC_Icon _aswbp_dialogue_3) "Visible")
    (Widget|SetVisibility (Variables|/Game/Assets/UI/Widgets/Dialogue/WBP_Dialogue.WBP_Dialogue_C|GetPlayer_Icon _aswbp_dialogue_3) "Hidden")
    (else
      (bind _aswbp_dialogue_4 (Utilities|Casting|CastToWBP_Dialogue _dialoguewidget))
      (Widget|SetVisibility (Variables|/Game/Assets/UI/Widgets/Dialogue/WBP_Dialogue.WBP_Dialogue_C|GetNPC_Icon _aswbp_dialogue_4) "Hidden")
      (Widget|SetVisibility (Variables|/Game/Assets/UI/Widgets/Dialogue/WBP_Dialogue.WBP_Dialogue_C|GetPlayer_Icon _aswbp_dialogue_4) "Visible"))))

(event EventBeginPlay
  (for (_ _array_index) (Variables|Default|GetConversationsList)
    (switch int _array_index
      (:0
        (Class|NPC|SetConversationQuest _array_index (Variables|Default|GetQuest0Objective)))
      (:1
        (Class|NPC|SetConversationQuest _array_index (Variables|Default|GetQuestObjective1)))
      (:2
        (Class|NPC|SetConversationQuest _array_index (Variables|Default|GetQuestObjective3))))))

(event Event_FinishQuest
  (bind _asbp_player_character (Utilities|Casting|CastToBP_PlayerCharacter (Game|GetPlayerCharacter 0)))
  (bind _returnvalue (Class|NPC|GetCurrentFishboneReward))
  (Variables|/Script/Catastrophe_VS.PlayerCharacter|SetFishBonesAmount _asbp_player_character (+ (Variables|/Script/Catastrophe_VS.PlayerCharacter|GetFishBonesAmount _asbp_player_character) _returnvalue)))

(event Event_Interact)

(fn ConstructionScript)