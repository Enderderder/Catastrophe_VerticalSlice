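; BP_FallingCrates is a one-shot interactable stack of crates that falls when the player interacts with it.
; Interaction sets the Fallen flag on the ABP_StackedCrates animation Blueprint, removes the outline and ends the interaction, which then disables the actor's interactivity.
; A blocking collider, off at BeginPlay, is enabled by a short timer after the fall starts.
; The overlap events are empty leftovers, alongside unconnected nodes.
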(event OnComponentBeginOverlap(BaseCollider)
  (params (OverlappedComponent :type Primitive%20Component%20Object%20Reference) (OtherActor :type Actor%20Object%20Reference) (OtherComp :type Primitive%20Component%20Object%20Reference) (OtherBodyIndex :type Integer) (bFromSweep :type Boolean) (SweepResult :type Hit%20Result%20Structure%20%28by%20ref%29))
  ;[1 1 1] Depracated
)

(event OnComponentEndOverlap(BaseCollider)
  (params (OverlappedComponent :type Primitive%20Component%20Object%20Reference) (OtherActor :type Actor%20Object%20Reference) (OtherComp :type Primitive%20Component%20Object%20Reference) (OtherBodyIndex :type Integer))
  ;[1 1 1] Depracated
)

(event EventReciveInteractionStart
  ;[1 1 1] On Interaction Start Event
  (bind _asabp_stacked_crates (Utilities|Casting|CastToABP_StackedCrates (Components|SkeletalMesh|GetAnimInstance (Variables|Default|GetMesh))))
  (Variables|/Game/Assets/StackedCrates/ABP_StackedCrates.ABP_StackedCrates_C|SetbFallen _asabp_stacked_crates true)
  (Utilities|Time|SetTimerbyFunctionName 0 "SpawnCollider" 0.4)
  (Components|DestroyComponent (Variables|Default|GetOutline))
  (Class|InteractActor|EndInteraction))

(event EventReciveInteractionEnd
  ;[1 1 1] On Interaction End Event
  (Class|InteractActor|DisableInteractActor))

(event EventBeginPlay
  ;[1 1 1] Disable the blocking collision
  (Collision|SetCollisionEnabled (Variables|Default|GetBlockedCollider) "NoCollision"))

(fn ConstructionScript)

(fn SpawnCollider
  (Collision|SetCollisionEnabled (Variables|Default|GetBlockedCollider) "QueryAndPhysics"))