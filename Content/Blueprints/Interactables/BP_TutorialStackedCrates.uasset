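; BP_TutorialStackedCrates is an interactable stacked-crates actor that serves as a tutorial quest objective.
; When the player interacts with it, it completes its QuestObjective.
; It listens to the objective's activate and complete events and prints the short description to screen as a new or completed task message.
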(event OnObjectiveActivate(QuestObjective)
  ;[1 1 1] Print to screen when QuestObjective is activated/completed
  (Development|PrintString (Utilities|String|Append "New Task: " (Variables|/Script/Catastrophe_VS.QuestObjectiveComponent|GetShortDescription (Variables|Default|GetQuestObjective)))))

(event OnObjectiveComplete(QuestObjective)
  ;[1 1 1] Print to screen when QuestObjective is activated/completed
  (Development|PrintString (Utilities|String|Append "Task Completed: " (Variables|/Script/Catastrophe_VS.QuestObjectiveComponent|GetShortDescription (Variables|Default|GetQuestObjective)))))

(event EventBeginPlay
  (|CallParentFunction) ; This node is disabled and will not be called.\nDrag off pins to build functionality.
)

(event Collision|EventActorBeginOverlap
  (params (OtherActor :type Actor%20Object%20Reference)))

(event EventTick
  (params (DeltaSeconds :type Float%20%28single-precision%29)))

(event Event_OnPlayerInteract
  ;[1 1 1] Complete Objective when interact
  (Class|QuestObjectiveComponent|CompleteObjective (Variables|Default|GetQuestObjective)))

(fn ConstructionScript
  (|CallParentFunction))