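; BP_JailUrn is a quest-linked interactable urn the player can jump into during a jail sequence.
; Each Tick, the quest objective's active state sets CanInteract and shows or hides the objective marker.
; On objective activation, it creates a quest-unlocked widget, stores it on the player character and updates it with the objective.
; Jumping in plays the guard-opening-cell level sequence and completes the objective.
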(event OnObjectiveActivate(QuestObjective)
  ;[1 1 1] Print to screen when Quests activated/completed
  (bind _asbp_player_character (Utilities|Casting|CastToBP_PlayerCharacter (Game|GetPlayerCharacter 0)))
  (bind _returnvalue (UserInterface|CreateWidget "/Game/Assets/UI/Widgets/Quests/WBP_QuestUnlocked.WBP_QuestUnlocked_C"))
  (UserInterface|Viewport|AddtoViewport _returnvalue 0)
  (bind _output_get (Variables|/Game/Blueprints/Characters/BP_PlayerCharacter.BP_PlayerCharacter_C|SetQuestWidget _asbp_player_character _returnvalue))
  (Default|Update _output_get (Variables|Default|GetQuestObjective)))

(event OnObjectiveComplete(QuestObjective)
  ;[1 1 1] Print to screen when Quests activated/completed
)

(event EventBeginPlay
  (|CallParentFunction) ; This node is disabled and will not be called.\nDrag off pins to build functionality.
)

(event Collision|EventActorBeginOverlap
  (params (OtherActor :type Actor%20Object%20Reference)))

(event Event_JumpIn
  (params (_playerCharacter :type Player%20Character%20Object%20Reference))
  (bind _returnvalue (Sequencer|Player|CreateLevelSequencePlayer "/Game/Sequences/S_GuardOpeningCell.S_GuardOpeningCell"))
  (Sequencer|Player|Play _returnvalue :!class /Script/MovieScene.MovieSceneSequencePlayer)
  (Class|QuestObjectiveComponent|CompleteObjective (Variables|Default|GetQuestObjective)))

(event EventTick
  (params (DeltaSeconds :type Float%20%28single-precision%29))
  (bind _output_get (Variables|Default|SetbCanInteract (Class|QuestObjectiveComponent|IsObjectiveActive (Variables|Default|GetQuestObjective))))
  (if _output_get
    (Rendering|SetVisibility (Variables|Default|GetObjectiveMarker) true false)
    (else
      (Rendering|SetVisibility (Variables|Default|GetObjectiveMarker) false false))))

(fn ConstructionScript
  (|CallParentFunction))