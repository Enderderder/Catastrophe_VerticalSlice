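; Jail exit trigger actor that opens the way out by destroying its Door component when the player reaches it.
; The trigger box starts with collision disabled, and RecieveSetDoorActive(true) enables it and hides the text render.
; A BP_PlayerCharacter overlap calls ReceiveActivateDoorTrigger, while the separate _ActivateDoorTrigger event performs the door destruction.
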(event OnComponentBeginOverlap(TriggerBox)
  (params (OverlappedComponent :type Primitive%20Component%20Object%20Reference) (OtherActor :type Actor%20Object%20Reference) (OtherComp :type Primitive%20Component%20Object%20Reference) (OtherBodyIndex :type Integer) (bFromSweep :type Boolean) (SweepResult :type Hit%20Result%20Structure%20%28by%20ref%29))
  ;[1 1 1] OnTriggerBeginOverlap
  (Utilities|Casting|CastToBP_PlayerCharacter OtherActor)
  (Class|DoorTrigger|ReceiveActivateDoorTrigger))

(event EventRecieveSetDoorActive
  (params (_b :type Boolean))
  (if _b
    (Collision|SetCollisionEnabled (Variables|Default|GetTriggerBox) "QueryAndPhysics")
    (Rendering|SetVisibility (Variables|Default|GetTextRender) false false)
    (else
      (Collision|SetCollisionEnabled (Variables|Default|GetTriggerBox) "NoCollision"))))

(event Event_ActivateDoorTrigger
  ;[1 1 1] Door Collision
  (Actor|DestroyActor (Variables|Default|GetDoor)))

(event EventBeginPlay
  (Class|DoorTrigger|RecieveSetDoorActive false))

(fn ConstructionScript)