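; Door trigger Blueprint that moves the player to the Market level.
; Its trigger box starts with collision off on BeginPlay, and SetDoorActive toggles that collision, though nothing in this graph re-enables it.
; When BP_PlayerCharacter overlaps the active box, it calls ReceiveActivateDoorTrigger, while the ActivateDoorTrigger event handler opens the hardcoded level by name.
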(event OnComponentBeginOverlap(TriggerBox)
  (params (OverlappedComponent :type Primitive%20Component%20Object%20Reference) (OtherActor :type Actor%20Object%20Reference) (OtherComp :type Primitive%20Component%20Object%20Reference) (OtherBodyIndex :type Integer) (bFromSweep :type Boolean) (SweepResult :type Hit%20Result%20Structure%20%28by%20ref%29))
  ;[1 1 1] OnTriggerBeginOverlap
  (Utilities|Casting|CastToBP_PlayerCharacter OtherActor)
  (Class|DoorTrigger|ReceiveActivateDoorTrigger))

(event Event_ActivateDoorTrigger
  ;[1 1 1] Door Collision
  (Game|OpenLevel(byName) "Market"))

(event EventBeginPlay
  (CallFunction|SetDoorActive false))

(fn ConstructionScript)

(fn SetDoorActive
  (params (doorActive :type Boolean))
  (if doorActive
    (Collision|SetCollisionEnabled (Variables|Default|GetTriggerBox) "QueryAndPhysics")
    (else
      (Collision|SetCollisionEnabled (Variables|Default|GetTriggerBox) "NoCollision"))))