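; Spline-based placement actor that lines a spline with copies of the Lightsingle static mesh using an alert material instance.
; The Construction Script divides the spline length by Spacing and adds a mesh component at each interval in local space, with fixed rotation and unit scale.
; The Event Graph has no active logic, so the actor does all its work at construction.
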(event EventBeginPlay)

(event Collision|EventActorBeginOverlap
  (params (OtherActor :type Actor%20Object%20Reference)))

(event EventTick
  (params (DeltaSeconds :type Float%20%28single-precision%29)))

(fn ConstructionScript
  (bind _splinecomponentexample (Variables|Default|GetSplineComponentExample))
  (bind _spacing (Variables|Default|Getspacing))
  (for _index (range 0 (.ReturnValue (Math|Float|Division(WholeandRemainder) (Spline|GetSplineLength _splinecomponentexample) _spacing)))
    (bind _returnvalue (AddComponent|AddStaticMeshComponent false (Math|Transform|MakeTransform (Spline|GetLocationatDistanceAlongSpline _splinecomponentexample (* _index _spacing) "Local"))))
    (Components|StaticMesh|SetStaticMesh _returnvalue "/Game/Assets/Props/lightsingle.lightsingle")
    (Rendering|Material|SetMaterial _returnvalue 0 "/Game/Assets/Props/Alert_mat_Inst_3.Alert_mat_Inst_3")))